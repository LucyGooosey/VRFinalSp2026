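; BP_Blender is a blender actor that teleports the player once it holds the required amount of coffee.
; Every Tick it compares the number of overlapping BP_coffee actors against Counting.
; On an exact match it sets Teleport, waits through a Delay, then moves the player pawn to the TeleportLocation actor, with debug prints along the way.
; The check has no one-shot guard, so teleports repeat while the count matches.
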(event `self.ReceiveActorBeginOverlap`
  (params (OtherActor :type "Actor Object Reference")))

(event `self.ReceiveTick`
  (params (DeltaSeconds :type "Float (single-precision)"))
  (`/Engine/EditorBlueprintResources/StandardMacros.CompareInt` (`KismetArrayLibrary.Array_Length` (`self.GetOverlappingActors` "/Game/BluePrint/BP_coffee.BP_coffee_C")) (`self.counting`)
    (:`==`
      (`KismetSystemLibrary.PrintString` " coffee")
      (bind _output_get (set `self.teleport` true))
      (if _output_get
        (`KismetSystemLibrary.PrintString` "start moving")
        (`KismetSystemLibrary.Delay` 5.0)
        (`KismetSystemLibrary.PrintString` "end delay")
        (`self.K2_SetActorLocation` (`GameplayStatics.GetPlayerPawn` 0) (`self.K2_GetActorLocation` (`self.teleportLocation`)) false true)))))

(fn `UserConstructionScript`)