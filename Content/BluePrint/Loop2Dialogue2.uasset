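; Blueprint that shows day 3 dialogue text on the VR pawn's dialogue widget through a Dialogue1 event.
; While the pawn's DialogueOn is set, each call increments an index into DialogueDay3, and clears the widget once the index exceeds the array length.
; The DialogueLook widget is created and given text only while UI is invalid, so later calls don't refresh the line.
; When DialogueOn is off, the widget is cleared.
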(event `/Game/VR_Dialogue.Dialogue1`
  (`KismetSystemLibrary.PrintString` "inDialogue1")
  (bind _asvrpawn (cast `/Game/VRTemplate/Blueprints/VRPawn` (`GameplayStatics.GetPlayerPawn` 0)))
  (if (`/Game/VRTemplate/Blueprints/VRPawn.dialogueOn` _asvrpawn)
    (`/Engine/EditorBlueprintResources/StandardMacros.IncrementInt` (`self.Dialogue_D2_Index`)
      (:`  `
        (if (<= (`self.Dialogue_D2_Index`) (`KismetArrayLibrary.Array_Length` (`self.Dialogue_Day3`)))
          (`self.UI`
            (:`then`)
            (:`else`
              (`KismetSystemLibrary.PrintString` "READ VALUE OF ui")
              (bind _returnvalue (`|CreateWidget` "/Game/DialogueLook.DialogueLook_C" (`GameplayStatics.GetPlayerController` 0)))
              (`KismetSystemLibrary.PrintString` "created UI")
              (bind _output_get (set `self.UI` _returnvalue))
              (bind _asvrpawn_2 (cast `/Game/VRTemplate/Blueprints/VRPawn` (`GameplayStatics.GetPlayerPawn` 0)))
              (`WidgetComponent.SetWidget` (`/Game/VRTemplate/Blueprints/VRPawn.DialogueWIdget` _asvrpawn_2) _output_get)
              (`KismetSystemLibrary.PrintString` "set widget")
              (`TextBlock.SetText` (`/Game/DialogueLook.Talking1` (`self.UI`)) (`KismetTextLibrary.Conv_StringToText` (`|GetArrayItem` (`self.Dialogue_Day3`) (`self.Dialogue_D2_Index`))))))
          (else
            (bind _asvrpawn_3 (cast `/Game/VRTemplate/Blueprints/VRPawn` (`GameplayStatics.GetPlayerPawn` 0) :!label _label))
            (`WidgetComponent.SetWidget` (`/Game/VRTemplate/Blueprints/VRPawn.DialogueWIdget` _asvrpawn_3) null)))))
    (else
      (goto _label))))

(fn `UserConstructionScript`
  (`parent.UserConstructionScript`))