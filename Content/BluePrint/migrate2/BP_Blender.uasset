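; BP_Blender is a blender actor that teleports the player once three coffee items are placed in it.
; Each Tick it counts overlapping BP_coffee actors and, at exactly three, sets the Teleport flag and moves player pawn 0 to a hard-coded location.
; The TeleportLocation actor's position appears only in a debug print, and the move repeats every frame while the count stays at three.
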(event `self.ReceiveActorBeginOverlap`
  (params (OtherActor :type "Actor Object Reference")))

(event `self.ReceiveTick`
  (params (DeltaSeconds :type "Float (single-precision)"))
  (bind _returnvalue (`GameplayStatics.GetPlayerPawn` 0))
  (`/Engine/EditorBlueprintResources/StandardMacros.CompareInt` (`KismetArrayLibrary.Array_Length` (`self.GetOverlappingActors` "/Game/BluePrint/migrate2/BP_coffee.BP_coffee_C")) 3
    (:`==`
      (`KismetSystemLibrary.PrintString` "3 coffee")
      (bind _output_get (set `self.teleport` true))
      (if _output_get
        (`KismetSystemLibrary.PrintString` "start moving")
        (`KismetSystemLibrary.PrintString` (`KismetStringLibrary.Concat_StrStr` (`KismetStringLibrary.Concat_StrStr` (`KismetSystemLibrary.GetObjectName` _returnvalue) "to") (`KismetStringLibrary.Conv_VectorToString` (`self.K2_GetActorLocation` (`self.teleportLocation`)))))
        (`self.K2_SetActorLocation` _returnvalue (-141520.218706 -7060.030689 -1763.475828) false true)))))

(fn `UserConstructionScript`)